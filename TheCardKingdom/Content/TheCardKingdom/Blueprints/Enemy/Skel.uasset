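; Skeleton enemy actor that walks a waypoint path to an end position and destroys itself when its HP runs out.
; BeginPlay appends the end position to the path, then Tick moves toward the first waypoint at constant speed, scaled by a multiplier.
; Movement is locked to a fixed X plane, so arrival compares only Y and Z before removing that waypoint.
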(event `self.ReceiveBeginPlay`
  (set `self.CurrentPosition` (`self.K2_GetActorLocation`))
  (`KismetArrayLibrary.Array_Add` (`self.Path`) (`self.EndPosition`))
  (for _array_element (`self.Path`)
    _))

(event `self.ReceiveTick`
  (params (DeltaSeconds :type "Float (single-precision)"))
  (`|ExecutionSequence`
    (:`then_0`
      (`self.MoveToTarget` DeltaSeconds (`|GetArrayItem` (`self.Path`)))
      (if (== (`KismetMathLibrary.MakeVector` 82.316917 (.y (`self.CurrentPosition`)) (.z (`self.CurrentPosition`))) (`KismetMathLibrary.MakeVector` 82.316917 (.y (`|GetArrayItem` (`self.Path`))) (.z (`|GetArrayItem` (`self.Path`)))))
        (`KismetArrayLibrary.Array_Remove` (`self.Path`))))
    (:`then_1`
      (`self.CheckDeath`))))

(fn `CheckDeath`
  (if (<= (`self.HP`) 0)
    (`self.K2_DestroyActor`)))

(fn `MoveToTarget`
  (params (FrameTime :type "Float (double-precision)") (TargetPos :type "Vector Structure"))
  (set `self.FrameTime` FrameTime)
  (bind _output_get (set `self.CurrentPosition` (`KismetMathLibrary.VInterpTo_Constant` (`self.CurrentPosition`) TargetPos (`self.FrameTime`) (* (`self.MovementSpeed`) (`self.SpeedMultiplier`)))))
  (`self.K2_SetActorLocation` (`KismetMathLibrary.MakeVector` 87.0 (.y _output_get) (.z _output_get))))

(fn `Test`
  (params (`Move here` :type "Vector Structure")))

(fn `UserConstructionScript`)