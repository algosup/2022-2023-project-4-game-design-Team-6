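; UtilityLib is a utility function library for The Card Kingdom with timing, card-array and sorting helpers.
; TrueOnX adds delta time to a caller-held timer, returning the new time and whether at least one full wait interval has elapsed, without resetting it.
; CardArray simply returns a Cards array.
; SortArray uses a swap-flag bubble sort to order elements by descending DistanceFromStart.
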(fn `CardArray`
  (returns (CardArray :type "Array of /Game/TheCardKingdom/Blueprints/Cards/Variables/Card_Struct Structure"))
  (locals (Cards :type "Array of /Game/TheCardKingdom/Blueprints/Cards/Variables/Card_Struct Structure"))
  (return (`local.Cards`)))

(fn `SortArray`
  (params (Unsorted :type "Array of /Game/TheCardKingdom/Blueprints/Board/Case Object Reference"))
  (returns (Sorted :type "Array of /Game/TheCardKingdom/Blueprints/Board/Case Object Reference"))
  (locals (Length :type Integer) (swapped :type Boolean :default true) (TempArray :type "Array of /Game/TheCardKingdom/Blueprints/Board/Case Object Reference"))
  (bind _temparray (`local.TempArray`))
  (bind _output_get (set `local.TempArray` Unsorted))
  (set `local.Length` (`KismetArrayLibrary.Array_Length` _output_get))
  (while (`local.swapped`)
    (set `local.swapped` false)
    (for _index (range 1 (`local.Length`))
      (if (< (`/Game/TheCardKingdom/Blueprints/Board/Case.DistanceFromStart` (`|GetArrayItem` _temparray (- _index 1))) (`/Game/TheCardKingdom/Blueprints/Board/Case.DistanceFromStart` (`|GetArrayItem` _temparray _index)))
        (set `local.swapped` true)
        (`KismetArrayLibrary.Array_Swap` (`local.TempArray`) _index (- _index 1)))))
  (return (`local.TempArray`)))

(fn `TrueOnX`
  (params (`Delta Seconds` :type "Float (double-precision)") (WaitTime :type "Float (double-precision)") (CurrentTime :type "Float (double-precision)"))
  (returns (Go :type Boolean) (NewCurrentTime :type "Float (double-precision)"))
  (locals (TimeFromStart :type "Float (double-precision)" :default 0.0))
  (bind _returnvalue (`KismetSystemLibrary.MakeLiteralDouble` WaitTime))
  (bind _output_get (set `local.TimeFromStart` CurrentTime))
  (bind _output_get_2 (set `local.TimeFromStart` (+ _output_get `Delta Seconds`)))
  (return (>= (- _output_get_2 (mod _output_get_2 _returnvalue)) _returnvalue) (`local.TimeFromStart`)))