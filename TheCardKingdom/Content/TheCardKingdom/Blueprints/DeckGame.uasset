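; Core game controller for a deck-building tower defense: runs turns, deck, hand, mana and castle HP.
; Tick switches on a phase: draw cards and save or load, place towers by spending mana, spawn skeletons on random tile paths, fight until none remain.
; Cards, tiles and the end-turn button are polled through GetAllActorsOfClass flags.
; Helpers record and respawn towers through the GI game instance, and zero castle HP returns to the main menu.
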(event `self.ReceiveBeginPlay`
  (set `self.ManaMax` (- (`self.ManaMax`) 1))
  (`self.ShuffleDeck`)
  (bind _asgi (cast `/Game/TheCardKingdom/Blueprints/Utility/GI` (`GameplayStatics.GetGameInstance`)))
  (set `self.As GI` _asgi))

(event `self.ReceiveTick`
  (params (DeltaSeconds :type "Float (single-precision)"))
  (bind _manamax (`self.ManaMax`))
  (bind _output (`|GetArrayItem` (`self.Towers`) (`|GetArrayItem` (`self.Hand`) (`self.SelectedCardIindex`))))
  (bind _returnvalue (`KismetMathLibrary.MakeTransform` (`KismetMathLibrary.MakeVector` (+ (.x (`self.TowerPosition`)) -1.0) (.y (`self.TowerPosition`)) (.z (`self.TowerPosition`)))))
  (bind _returnvalue_2 (- (`self.Mana`) (`.Mana_Cost_6_6E1F3F9E409D431BEDABBD934F20ABB1` (break `/Game/TheCardKingdom/Blueprints/Cards/Variables/Card_Struct` (`self.GetCardByID` (`|GetArrayItem` (`self.Hand`) (`self.SelectedCardIindex`)))))))
  (switch `/Game/TheCardKingdom/Blueprints/Utility/GameStates` (`self.CurrentPhase`)
    (:`NewEnumerator1`
      ;[0.4063 1 0.5617] On the start of a turn
      (`|ExecutionSequence`
        (:`then_0`
          (`self.Save&Load`))
        (:`then_1`
          (for _ (range 1 8)
            (`self.DrawCard`))
          (`self.RenderHand`))
        (:`then_2`
          ;;[1 1 1] Update mana (+1 mana max if not already max, and reset to max)
          (if (< _manamax 10)
            (set `self.ManaMax` (+ _manamax 1)))
          (set `self.Mana` (`self.ManaMax`)))
        (:`then_3`
          (set `self.CurrentPhase` "NewEnumerator2")
          (`self.SetEndSetup` false))
        (:`then_4`
          (bind _outactors (`GameplayStatics.GetAllActorsOfClass` "/Game/TheCardKingdom/Blueprints/Tower/ArcherTower.ArcherTower_C"))
          (for _array_element _outactors
            (`SceneComponent.K2_SetWorldTransform` (`/Game/TheCardKingdom/Blueprints/Tower/ArcherTower.Range` _array_element) (`KismetMathLibrary.MakeTransform` (0.0 0.0 0.0) (struct) (0.0 0.0 0.0)) false false)))
        (:`then_5`
          (if (<= (`self.CastleHP`) 0)
            (`GameplayStatics.DeleteGameInSlot` "Auto_Save")
            (`GameplayStatics.OpenLevelBySoftObjectPtr` "/Game/TheCardKingdom/Levels/MainMenu.MainMenu")))))
    (:`NewEnumerator2`
      ;[0.2954 0.8043 1] Setup Phase
      (`|ExecutionSequence`
        (:`then_1`
          ;;[1 1 1] Select a card
          (`|ExecutionSequence`
            (:`then_0`
              (`self.SelectCard`)
              (bind _index (`self.GetSelectedCard`))
              (set `self.SelectedCardIindex` _index))
            (:`then_1`
              (set `self.CardSelected` (`|GetArrayItem` (`/Game/TheCardKingdom/Blueprints/Utility/UtilityLib.CardArray`) (`|GetArrayItem` (`self.Hand`) (`self.SelectedCardIindex`)))))))
        (:`then_2`
          ;;[1 1 1] Card Selected
          (if (!= (`self.SelectedCardIindex`) -1)
            ;;[1 1 1] Want to place the card at a valid spot
            (bind (_clickedposition _activated _hasatower) (`self.GetFirstSquareClicked`))
            (if (and _activated (not _hasatower))
              (set `self.TowerPosition` _clickedposition)
              ;;[1 1 1] Place the selected card on the board
              ;;;[1 1 1] Enough Mana && Update mana
              (if (>= _returnvalue_2 0)
                (set `self.Mana` _returnvalue_2)
                ;;;[1 1 1] Spawn tower
                (if (`KismetSystemLibrary.IsValidClass` _output)
                  (`|SpawnActorFromClass` _output _returnvalue "Undefined" "OverrideRootScale" null null)
                  (else
                    (`|SpawnActorFromClass` "/Game/TheCardKingdom/Blueprints/Tower/AAAAAAAAAA.AAAAAAAAAA_C" _returnvalue "Undefined" "OverrideRootScale" null null)))
                (`self.DiscardCard` (`self.SelectedCardIindex`))))))
        (:`then_3`
          ;;[1 1 1] Update the scene HUD
          (`|ExecutionSequence`
            (:`then_0`
              (bind _outactors_2 (`GameplayStatics.GetAllActorsOfClass` "/Game/TheCardKingdom/Blueprints/Utility/ManaCounter.ManaCounter_C"))
              (for _array_element_2 _outactors_2
                (`TextRenderComponent.K2_SetText` (`/Game/TheCardKingdom/Blueprints/Utility/ManaCounter.Mana_Current` _array_element_2) (`KismetTextLibrary.Conv_Int64ToText` (`self.Mana`)))
                (`TextRenderComponent.K2_SetText` (`/Game/TheCardKingdom/Blueprints/Utility/ManaCounter.Mana_Max` _array_element_2) (`KismetTextLibrary.Conv_Int64ToText` (`self.ManaMax`)))))
            (:`then_1`
              (bind _outactors_3 (`GameplayStatics.GetAllActorsOfClass` "/Game/TheCardKingdom/Blueprints/Utility/DeckCardCounter.DeckCardCounter_C"))
              (for _array_element_3 _outactors_3
                (`TextRenderComponent.K2_SetText` (`/Game/TheCardKingdom/Blueprints/Utility/DeckCardCounter.NbCards` _array_element_3) (`KismetTextLibrary.Conv_IntToText` (`KismetArrayLibrary.Array_Length` (`self.Deck`))))))
            (:`then_2`
              (bind _outactors_4 (`GameplayStatics.GetAllActorsOfClass` "/Game/TheCardKingdom/Blueprints/Utility/DiscardCardCounter.DiscardCardCounter_C"))
              (for _array_element_4 _outactors_4
                (`TextRenderComponent.K2_SetText` (`/Game/TheCardKingdom/Blueprints/Utility/DiscardCardCounter.NbCards` _array_element_4) (`KismetTextLibrary.Conv_IntToText` (`KismetArrayLibrary.Array_Length` (`self.Discard`))))))))
        (:`then_4`
          ;;[1 1 1] Get the end turn button state
          (bind _endphase (`self.GetEndSetup`))
          (if _endphase
            (set `self.CurrentPhase` "NewEnumerator3")))))
    (:`NewEnumerator3`
      ;[1 0.2948 0.3037] Setup Battle
      ;;[1 0.7418 0.5719] End turn, discard all cards
      (`|ExecutionSequence`
        (:`then_0`
          (while (> (`KismetArrayLibrary.Array_Length` (`self.Hand`)) 0)
            (`self.DiscardCard` 0)))
        (:`then_1`
          (`self.HideTowerRange`)
          (set `self.WaveID` (+ (`self.WaveID`) 1)))
        (:`then_2`
          ;;[1 1 1] Comment
          (`|ExecutionSequence`
            (:`then_0`
              (bind _returnvalue_3 (`GameplayStatics.GetActorOfClass` "/Game/TheCardKingdom/Blueprints/Utility/SpawnZone.SpawnZone_C"))
              (set `self.SpawnPoint` (.location (`self.GetTransform` _returnvalue_3))))
            (:`then_1`
              (bind _outactors_5 (`GameplayStatics.GetAllActorsOfClass` "/Game/TheCardKingdom/Blueprints/Board/Case.Case_C"))
              (for _ (range 7)
                (`KismetArrayLibrary.Array_Add` (`self.Path`) (`self.K2_GetActorLocation` (`KismetArrayLibrary.Array_Random` _outactors_5))))
              (bind _returnvalue_4 (`GameplayStatics.GetActorOfClass` "/Game/TheCardKingdom/Blueprints/Utility/EndZone.EndZone_C"))
              (`KismetArrayLibrary.Array_Add` (`self.Path`) (`self.K2_GetActorLocation` _returnvalue_4)))
            (:`then_2`
              (bind _returnvalue_5 (`GameplayStatics.GetActorOfClass` "/Game/TheCardKingdom/Blueprints/Utility/EndZone.EndZone_C"))
              ;;;[1 1 1] For each enemy in the wave
              (for _ (range (+ (`KismetMathLibrary.Conv_Int64ToInt` (* (`self.ManaMax`) 3)) 1))
                (`|SpawnActorFromClass` "/Game/TheCardKingdom/Blueprints/Enemy/Skel.Skel_C" (`KismetMathLibrary.MakeTransform` (`KismetMathLibrary.MakeVector` 5.55 (.y (`self.SpawnPoint`)) (.z (`self.SpawnPoint`)))) "Undefined" "OverrideRootScale" null (`self.Path`) (`self.K2_GetActorLocation` _returnvalue_5) 40 5 null)))
            (:`then_3`
              (set `self.CurrentPhase` "NewEnumerator4"))))))
    (:`NewEnumerator4`
      ;[1 1 1] End battle phase when no ennemy remains
      (bind _outactors_6 (`GameplayStatics.GetAllActorsOfClass` "/Game/TheCardKingdom/Blueprints/Enemy/Skel.Skel_C"))
      (if (<= (`KismetArrayLibrary.Array_Length` _outactors_6) 0)
        (set `self.CurrentPhase` "NewEnumerator1")
        (else
          (bind _returnvalue_6 (`GameplayStatics.GetActorOfClass` "/Game/TheCardKingdom/Blueprints/Utility/EndZone.EndZone_C"))
          (for _array_element_5 _outactors_6
            (if (== (`KismetMathLibrary.MakeVector` 0.0 (.y (`self.K2_GetActorLocation` _array_element_5)) (.z (`self.K2_GetActorLocation` _array_element_5))) (`KismetMathLibrary.MakeVector` 0.0 (.y (`self.K2_GetActorLocation` _returnvalue_6)) (.z (`self.K2_GetActorLocation` _returnvalue_6))) :`ErrorTolerance` 0.001)
              (`|ExecutionSequence`
                (:`then_0`
                  (set `self.CastleHP` (- (`self.CastleHP`) (`/Game/TheCardKingdom/Blueprints/Enemy/Skel.Damage` _array_element_5)))
                  (`self.K2_DestroyActor` _array_element_5))
                (:`then_1`)
                (:`then_2`)))))))))

(fn `DiscardCard`
  (params (Index :type Integer))
  (`KismetArrayLibrary.Array_Add` (`self.Discard`) (`|GetArrayItem` (`self.Hand`) Index))
  (`KismetArrayLibrary.Array_Remove` (`self.Hand`) Index)
  (`self.RenderHand`))

(fn `DrawCard`
  (locals (`Empty Array` :type "Array of Integer"))
  (bind _hand (`self.Hand`))
  (if (> (`KismetArrayLibrary.Array_Length` (`self.Deck`)) 0)
    (`KismetArrayLibrary.Array_Insert` _hand (`|GetArrayItem` (`self.Deck`)) (`KismetArrayLibrary.Array_Length` _hand) :!label _label)
    (`KismetArrayLibrary.Array_Remove` (`self.Deck`))
    (else
      (`KismetArrayLibrary.Array_Shuffle` (`self.Discard`))
      (set `self.Deck` (`self.Discard`))
      (set `self.Discard` (`local.Empty Array`))
      (if (> (`KismetArrayLibrary.Array_Length` (`self.Deck`)) 0)
        (goto _label)))))

(fn `Get All Towers`
  (bind _as_gi (`self.As GI`))
  (bind _returnvalue (`KismetArrayLibrary.Array_Length` (`/Game/TheCardKingdom/Blueprints/Utility/GI.GI_TowersID` (`self.As GI`))))
  (`KismetArrayLibrary.Array_Clear` (`/Game/TheCardKingdom/Blueprints/Utility/GI.GI_TowersTransform` _as_gi))
  (`KismetArrayLibrary.Array_Clear` (`/Game/TheCardKingdom/Blueprints/Utility/GI.GI_TowersID` _as_gi))
  (bind _outactors (`GameplayStatics.GetAllActorsOfClass` "/Game/TheCardKingdom/Blueprints/Tower/ArcherTower.ArcherTower_C"))
  (for (_array_element _array_index) _outactors
    (`KismetArrayLibrary.Array_Set` (`/Game/TheCardKingdom/Blueprints/Utility/GI.GI_TowersID` (`self.As GI`)) _array_index 0 true)
    (`KismetArrayLibrary.Array_Set` (`/Game/TheCardKingdom/Blueprints/Utility/GI.GI_TowersTransform` (`self.As GI`)) _array_index (`self.GetTransform` _array_element) true))
  (bind _outactors_2 (`GameplayStatics.GetAllActorsOfClass` "/Game/TheCardKingdom/Blueprints/Tower/CrossbowTower.CrossbowTower_C"))
  (for _array_element_2 _outactors_2
    (`KismetArrayLibrary.Array_Set` (`/Game/TheCardKingdom/Blueprints/Utility/GI.GI_TowersID` (`self.As GI`)) _returnvalue 1 true)
    (`KismetArrayLibrary.Array_Set` (`/Game/TheCardKingdom/Blueprints/Utility/GI.GI_TowersTransform` (`self.As GI`)) (`KismetArrayLibrary.Array_Length` (`/Game/TheCardKingdom/Blueprints/Utility/GI.GI_TowersTransform` (`self.As GI`))) (`self.GetTransform` _array_element_2) true))
  (bind _outactors_3 (`GameplayStatics.GetAllActorsOfClass` "/Game/TheCardKingdom/Blueprints/Tower/CrystalTower.CrystalTower_C"))
  (for _array_element_3 _outactors_3
    (`KismetArrayLibrary.Array_Set` (`/Game/TheCardKingdom/Blueprints/Utility/GI.GI_TowersID` (`self.As GI`)) _returnvalue 2 true)
    (`KismetArrayLibrary.Array_Set` (`/Game/TheCardKingdom/Blueprints/Utility/GI.GI_TowersTransform` (`self.As GI`)) (`KismetArrayLibrary.Array_Length` (`/Game/TheCardKingdom/Blueprints/Utility/GI.GI_TowersTransform` (`self.As GI`))) (`self.GetTransform` _array_element_3) true))
  (bind _outactors_4 (`GameplayStatics.GetAllActorsOfClass` "/Game/TheCardKingdom/Blueprints/Tower/DisruptorTower.DisruptorTower_C"))
  (for _array_element_4 _outactors_4
    (`KismetArrayLibrary.Array_Set` (`/Game/TheCardKingdom/Blueprints/Utility/GI.GI_TowersID` (`self.As GI`)) _returnvalue 3 true)
    (`KismetArrayLibrary.Array_Set` (`/Game/TheCardKingdom/Blueprints/Utility/GI.GI_TowersTransform` (`self.As GI`)) (`KismetArrayLibrary.Array_Length` (`/Game/TheCardKingdom/Blueprints/Utility/GI.GI_TowersTransform` (`self.As GI`))) (`self.GetTransform` _array_element_4) true)))

(fn `GetCardByID`
  (params (ID :type Integer))
  (returns (Output :type "/Game/TheCardKingdom/Blueprints/Cards/Variables/Card_Struct Structure"))
  (locals (Deck :type "Array of Integer"))
  (return (`|GetArrayItem` (`/Game/TheCardKingdom/Blueprints/Utility/UtilityLib.CardArray` null) ID)))

(fn `GetEndSetup`
  (returns (EndPhase :type Boolean))
  (bind _outactors (`GameplayStatics.GetAllActorsOfClass` "/Game/TheCardKingdom/Blueprints/Board/EndSetup.EndSetup_C"))
  (return (`/Game/TheCardKingdom/Blueprints/Board/EndSetup.EndPhase` (`|GetArrayItem` _outactors))))

(fn `GetFirstSquareClicked`
  (returns (ClickedPosition :type "Vector Structure") (Activated :type Boolean) (HasATower :type Boolean))
  (locals (Position :type "Vector Structure") (Active :type Boolean) (HasTower :type Boolean))
  (set `local.Position` (0.0 0.0 0.0))
  (set `local.Active` false)
  (bind _outactors (`GameplayStatics.GetAllActorsOfClass` "/Game/TheCardKingdom/Blueprints/Board/Case.Case_C"))
  (for _array_element _outactors
    (if (`/Game/TheCardKingdom/Blueprints/Board/Case.LastActivated` _array_element)
      (set `/Game/TheCardKingdom/Blueprints/Board/Case.LastActivated` false _array_element)
      (set `local.Position` (`self.K2_GetActorLocation` _array_element))
      (set `local.Active` true)
      (if (`/Game/TheCardKingdom/Blueprints/Board/Case.HasATower` _array_element)
        (set `local.HasTower` true)
        (`KismetSystemLibrary.PrintString` "Hello"))))
  (return (`local.Position`) (`local.Active`) (`local.HasTower`)))

(fn `GetSelectedCard`
  (returns (Index :type Integer))
  (locals (HandIndex :type Integer :default -1))
  (bind _outactors (`GameplayStatics.GetAllActorsOfClass` "/Game/TheCardKingdom/Blueprints/Cards/CardTemplate/CardActor.CardActor_C"))
  (for _array_element _outactors
    (if (`/Game/TheCardKingdom/Blueprints/Cards/CardTemplate/CardActor.Selected` _array_element)
      (set `local.HandIndex` (`/Game/TheCardKingdom/Blueprints/Cards/CardTemplate/CardActor.Index` _array_element))))
  (return (`local.HandIndex`)))

(fn `HideTowerRange`
  (`|ExecutionSequence`
    (:`then_0`
      (bind _outactors (`GameplayStatics.GetAllActorsOfClass` "/Game/TheCardKingdom/Blueprints/Tower/AAAAAAAAAA.AAAAAAAAAA_C"))
      (for _array_element _outactors
        (`SceneComponent.K2_SetWorldTransform` (`/Game/TheCardKingdom/Blueprints/Tower/AAAAAAAAAA.Range` _array_element) (`/Game/TheCardKingdom/Blueprints/Tower/AAAAAAAAAA.RangeTransform` _array_element) false false)))
    (:`then_1`
      (bind _outactors_2 (`GameplayStatics.GetAllActorsOfClass` "/Game/TheCardKingdom/Blueprints/Tower/ArcherTower.ArcherTower_C"))
      (for _array_element_2 _outactors_2
        (`SceneComponent.K2_SetWorldTransform` (`/Game/TheCardKingdom/Blueprints/Tower/ArcherTower.Range` _array_element_2) (`/Game/TheCardKingdom/Blueprints/Tower/ArcherTower.RangeTransform` _array_element_2) false false)))
    (:`then_2`
      (bind _outactors_3 (`GameplayStatics.GetAllActorsOfClass` "/Game/TheCardKingdom/Blueprints/Tower/CrossbowTower.CrossbowTower_C"))
      (for _array_element_3 _outactors_3
        (`SceneComponent.K2_SetWorldTransform` (`/Game/TheCardKingdom/Blueprints/Tower/CrossbowTower.Range` _array_element_3) (`/Game/TheCardKingdom/Blueprints/Tower/CrossbowTower.RangeTransform` _array_element_3) false false)))
    (:`then_3`
      (bind _outactors_4 (`GameplayStatics.GetAllActorsOfClass` "/Game/TheCardKingdom/Blueprints/Tower/CrystalTower.CrystalTower_C"))
      (for _array_element_4 _outactors_4
        (`SceneComponent.K2_SetWorldTransform` (`/Game/TheCardKingdom/Blueprints/Tower/CrystalTower.Range` _array_element_4) (`/Game/TheCardKingdom/Blueprints/Tower/CrystalTower.RangeTransform` _array_element_4) false false)))
    (:`then_4`
      (bind _outactors_5 (`GameplayStatics.GetAllActorsOfClass` "/Game/TheCardKingdom/Blueprints/Tower/DisruptorTower.DisruptorTower_C"))
      (for _array_element_5 _outactors_5
        (`SceneComponent.K2_SetWorldTransform` (`/Game/TheCardKingdom/Blueprints/Tower/DisruptorTower.Range` _array_element_5) (`/Game/TheCardKingdom/Blueprints/Tower/DisruptorTower.RangeTransform` _array_element_5) false false)))))

(fn `NewFunction_0`
  (bind _outactors (`GameplayStatics.GetAllActorsOfClass` "/Game/TheCardKingdom/Blueprints/Enemy/Skel.Skel_C"))
  (bind _returnvalue (`GameplayStatics.GetActorOfClass` "/Game/TheCardKingdom/Blueprints/Utility/EndZone.EndZone_C"))
  (for _array_element _outactors
    (if (== (`KismetMathLibrary.MakeVector` 0.0 (.y (`self.K2_GetActorLocation` _array_element)) (.z (`self.K2_GetActorLocation` _array_element))) (`KismetMathLibrary.MakeVector` 0.0 (.y (`self.K2_GetActorLocation` _returnvalue)) (.z (`self.K2_GetActorLocation` _returnvalue))))
      (set `self.CastleHP` (- (`self.CastleHP`) (`/Game/TheCardKingdom/Blueprints/Enemy/Skel.Damage` _array_element)))
      (`self.K2_DestroyActor`))))

(fn `RenderHand`
  (bind _outactors (`GameplayStatics.GetAllActorsOfClass` "/Game/TheCardKingdom/Blueprints/Cards/CardTemplate/CardActor.CardActor_C"))
  (for _array_element _outactors
    (`self.K2_DestroyActor` _array_element))
  (for (_array_element_2 _array_index) (`self.Hand`)
    (`|SpawnActorFromClass` "/Game/TheCardKingdom/Blueprints/Cards/CardTemplate/CardActor.CardActor_C" (`KismetMathLibrary.MakeTransform` (`KismetMathLibrary.MakeVector` (- (.x (.location (`KismetMathLibrary.MakeTransform` (200.0 25.0 -45.0) (struct) (0.2 0.2 0.2)))) (* _array_index 4.0)) (- (.y (.location (`KismetMathLibrary.MakeTransform` (200.0 25.0 -45.0) (struct) (0.2 0.2 0.2)))) (* _array_index (/ 60.0 (- (`KismetMathLibrary.Conv_IntToDouble` (`KismetArrayLibrary.Array_Length` (`self.Hand`))) 1.0)))) (.z (.location (`KismetMathLibrary.MakeTransform` (200.0 25.0 -45.0) (struct) (0.2 0.2 0.2))))) (.rotation (`KismetMathLibrary.MakeTransform` (200.0 25.0 -45.0) (struct) (0.2 0.2 0.2))) (.scale (`KismetMathLibrary.MakeTransform` (200.0 25.0 -45.0) (struct) (0.2 0.2 0.2)))) "Undefined" "OverrideRootScale" null _array_element_2 false false _array_index null)))

(fn `Save&Load`
  (bind _returnvalue (`GameplayStatics.GetCurrentLevelName` true))
  (if (`KismetStringLibrary.EqualEqual_StrStr` _returnvalue "BattlePhase")
    (bind _asgi (cast `/Game/TheCardKingdom/Blueprints/Utility/GI` (`GameplayStatics.GetGameInstance`)))
    (`/Game/TheCardKingdom/Blueprints/Utility/GI.GetContinue` _asgi)
    (if (== true (`/Game/TheCardKingdom/Blueprints/Utility/GI.continue` _asgi))
      (`/Game/TheCardKingdom/Blueprints/Utility/GI.Loading function` _asgi)
      (set `/Game/TheCardKingdom/Blueprints/Utility/GI.continue` false _asgi)
      (else
        (`/Game/TheCardKingdom/Blueprints/Utility/GI.Saving function` _asgi)))))

(fn `SelectCard`
  (locals (Hand_Index :type Integer :default -1))
  (bind _outactors (`GameplayStatics.GetAllActorsOfClass` "/Game/TheCardKingdom/Blueprints/Cards/CardTemplate/CardActor.CardActor_C"))
  (for _array_element _outactors
    (if (`/Game/TheCardKingdom/Blueprints/Cards/CardTemplate/CardActor.LastSelected` _array_element)
      (for _array_element_2 _outactors
        (if (`/Game/TheCardKingdom/Blueprints/Cards/CardTemplate/CardActor.LastSelected` _array_element_2)
          (set `/Game/TheCardKingdom/Blueprints/Cards/CardTemplate/CardActor.Selected` true _array_element_2)
          (else
            (set `/Game/TheCardKingdom/Blueprints/Cards/CardTemplate/CardActor.Selected` false _array_element_2)))
        (set `/Game/TheCardKingdom/Blueprints/Cards/CardTemplate/CardActor.LastSelected` false _array_element_2))
      (break))))

(fn `SetEndSetup`
  (params (`Set Value` :type Boolean))
  (returns (EndPhase :type Boolean))
  (bind _outactors (`GameplayStatics.GetAllActorsOfClass` "/Game/TheCardKingdom/Blueprints/Board/EndSetup.EndSetup_C"))
  (set `/Game/TheCardKingdom/Blueprints/Board/EndSetup.EndPhase` `Set Value` (`|GetArrayItem` _outactors))
  (return false))

(fn `ShuffleDeck`
  (`KismetArrayLibrary.Array_Shuffle` (`self.Deck`)))

(fn `SpawnReloadTowers`
  (`|ExecutionSequence`
    (:`then_0`
      (for (_array_element _array_index) (`/Game/TheCardKingdom/Blueprints/Utility/GI.GI_TowersID` (`self.As GI`))
        (`|SpawnActorFromClass` (`|GetArrayItem` (`self.Towers`) _array_element) (`|GetArrayItem` (`/Game/TheCardKingdom/Blueprints/Utility/GI.GI_TowersTransform` (`self.As GI`)) _array_index) "Undefined" "OverrideRootScale" null null)))))

(fn `UserConstructionScript`)